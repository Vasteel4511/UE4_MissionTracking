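; BP_RedThinger is a shootable objective actor made of three static meshes.
; Each mesh destroys itself when its hit event comes from a FirstPersonProjectile.
; BPIsObjectiveComplete reports completion once all three mesh components are no longer valid.
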(event `self.StaticMesh.OnComponentHit`
  (params (HitComponent :type "PrimitiveComponent Object Reference") (OtherActor :type "Actor Object Reference") (OtherComp :type "PrimitiveComponent Object Reference") (NormalImpulse :type "Vector Structure") (Hit :type "HitResult Structure (by ref)"))
  (cast `/Game/FirstPersonCPP/Blueprints/FirstPersonProjectile` OtherActor)
  (`ActorComponent.K2_DestroyComponent` (`self.StaticMesh`)))

(event `self.StaticMesh1.OnComponentHit`
  (params (HitComponent :type "PrimitiveComponent Object Reference") (OtherActor :type "Actor Object Reference") (OtherComp :type "PrimitiveComponent Object Reference") (NormalImpulse :type "Vector Structure") (Hit :type "HitResult Structure (by ref)"))
  (cast `/Game/FirstPersonCPP/Blueprints/FirstPersonProjectile` OtherActor)
  (`ActorComponent.K2_DestroyComponent` (`self.StaticMesh1`)))

(event `self.StaticMesh2.OnComponentHit`
  (params (HitComponent :type "PrimitiveComponent Object Reference") (OtherActor :type "Actor Object Reference") (OtherComp :type "PrimitiveComponent Object Reference") (NormalImpulse :type "Vector Structure") (Hit :type "HitResult Structure (by ref)"))
  (cast `/Game/FirstPersonCPP/Blueprints/FirstPersonProjectile` OtherActor)
  (`ActorComponent.K2_DestroyComponent` (`self.StaticMesh2`)))

(fn `BP_IsObjectiveComplete?`
  (returns (`?` :type Boolean))
  (return (and (not (`KismetSystemLibrary.IsValid` (`self.StaticMesh`))) (not (`KismetSystemLibrary.IsValid` (`self.StaticMesh1`))) (not (`KismetSystemLibrary.IsValid` (`self.StaticMesh2`))))))

(fn `UserConstructionScript`)