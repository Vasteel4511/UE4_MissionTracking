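; Actor component that tracks the current mission's progress through an ordered list of objectives.
; StartMission enables tracking, then Tick asks the first objective's tracking actor whether it is complete through an IsObjectiveCompleteMessage call.
; Completed objectives are removed from the front of the array, working as a queue.
; Each new objective and the final mission completion are reported only through log-only PrintString calls.
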(event `Start Mission`
  (set `self.HasMission?` true)
  (`self.Next Objective`))

(event `self.ReceiveTick`
  (params (DeltaSeconds :type "Float (single-precision)"))
  (bind (_currentmission_name _currentmission_objectives) (break `Mission` (`self.CurrentMission`)))
  (bind (_currentmission_name_2 _currentmission_objectives_2) (break `Mission` (`self.CurrentMission`)))
  (bind (_output_name _output_description _output_objectivetrackingactor) (break `Objective` (`|GetArrayItem` _currentmission_objectives_2)))
  (if (`self.HasMission?`)
    (if (> (`KismetArrayLibrary.Array_Length` _currentmission_objectives_2) 0)
      (`/Engine/EditorBlueprintResources/StandardMacros.IsValid` _output_objectivetrackingactor
        (:`Is Valid`
          (bind __ (message `/Game/BPI_ObjectiveTrack.BP_IsObjectiveComplete?` _output_objectivetrackingactor))
          (if __
            (`KismetArrayLibrary.Array_Remove` _currentmission_objectives)
            (if (> (`KismetArrayLibrary.Array_Length` _currentmission_objectives) 0)
              (`self.Next Objective`)
              (else
                (`KismetSystemLibrary.PrintString` "Mission Complete" false)))))))))

(event `Next Objective`
  (bind (_currentmission_name _currentmission_objectives) (break `Mission` (`self.CurrentMission`)))
  (bind (_output_name _output_description) (break `Objective` (`|GetArrayItem` _currentmission_objectives)))
  (`KismetSystemLibrary.PrintString` (`KismetStringLibrary.Concat_StrStr` "Mission: " (`KismetTextLibrary.Conv_TextToString` _currentmission_name) ", Current Objective: " (`KismetTextLibrary.Conv_TextToString` _output_name) ", Description: " (`KismetTextLibrary.Conv_TextToString` _output_description)) false))